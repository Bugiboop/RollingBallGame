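; Player-controlled rolling ball pawn that moves with physics, shoots bullets and rams forward.
; Movement axes apply camera-relative torque and force, while camera axes rotate the SpringArm with clamped pitch.
; Held Shoot loops on a short delay, launching bullets from the Cube with explosion effects and recoil on the ball.
; Ram is an impulse with sparks that clears CanJump, never reset here; hits push the struck component along the impact direction.
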(event Collision|EventHit
  (params (MyComp :type Primitive%20Component%20Object%20Reference) (Other :type Actor%20Object%20Reference) (OtherComp :type Primitive%20Component%20Object%20Reference) (bSelfMoved :type Boolean) (HitLocation :type Vector :default "0, 0, 0") (HitNormal :type Vector :default "0, 0, 0") (NormalImpulse :type Vector :default "0, 0, 0") (Hit :type Hit%20Result%20Structure%20%28by%20ref%29))
  (bind (_bblockinghit _binitialoverlap _time _distance _location _impactpoint _normal _impactnormal _physmat _hitactor _hitcomponent) (Collision|BreakHitResult Hit))
  (Physics|AddImpulse _hitcomponent (* (Math|Vector|GetUnitDirection(Vector) (Transformation|GetWorldLocation (Variables|Default|GetBall)) _location) (Variables|Default|GetBallHitForce)) "None" false))

(event Input|ActionEvents|InputActionRam
  (params (Key :type Key%20Structure))
  (:Pressed
    (if (Variables|Default|GetbCanJump)
      (Physics|AddImpulse (Variables|Default|GetBall) (* (Math|Vector|GetForwardVector (Transformation|GetWorldRotation (Variables|Default|GetCamera))) (Variables|Default|GetRamImpulse)) "None" false)
      (bind _returnvalue (Effects|SpawnEmitteratLocation "/Game/StarterContent/Particles/P_Sparks.P_Sparks" (Transformation|GetWorldLocation (Variables|Default|GetBall)) (Math|Rotator|MakeRotfromX (* (Math|Vector|GetForwardVector (Variables|Default|GetCamera)) -1)) "5.000000,5.000000,5.000000"))
      (Utilities|FlowControl|Delay 0.2)
      (Components|DestroyComponent _returnvalue)
      (Variables|Default|SetbCanJump false))))

(event Input|ActionEvents|InputActionShoot
  (params (Key :type Key%20Structure))
  (bind _camera (Variables|Default|GetCamera))
  (bind _cube (Variables|Default|GetCube))
  (bind _camera_2 (Variables|Default|GetCamera))
  (bind _returnvalue (Transformation|GetWorldTransform _cube))
  (bind _returnvalue_2 (Transformation|GetWorldRotation _camera))
  (bind _returnvalue_3 (Transformation|GetWorldRotation _camera_2))
  (:Pressed
    (Variables|Default|SetShootHeld true)
    (if (Variables|Default|GetShootHeld) :!label _label
      (bind _returnvalue_4 (Game|SpawnActorfromClass "/Game/Bullet.Bullet_C" (Math|Transform|MakeTransform (.location _returnvalue) (.rotation _returnvalue) "1,1,1") "AdjustIfPossibleButAlwaysSpawn" 0 0))
      (Physics|AddImpulse (Variables|/Script/Engine.StaticMeshActor|GetStaticMeshComponent _returnvalue_4) (* (Math|Vector|GetForwardVector (Math|Rotator|MakeRotator (.roll _returnvalue_3) (+ (.pitch _returnvalue_3) 15.0) (.yaw _returnvalue_3))) 5e+03) "None" true)
      (Effects|SpawnEmitterAttached "/Game/StarterContent/Particles/P_Explosion.P_Explosion" (Variables|Default|GetCube) "None" "0, 0, 0" "0, 0,0.000000")
      (Physics|AddImpulse (Variables|Default|GetBall) (* (Math|Vector|GetForwardVector (Math|Rotator|MakeRotator (.roll _returnvalue_2) (+ (.pitch _returnvalue_2) 15.0) (.yaw _returnvalue_2))) -2e+02) "None" true)
      (Utilities|FlowControl|Delay 0.1)
      (goto _label)))
  (:Released
    (Variables|Default|SetShootHeld false)
    (goto _label)))

(event Input|AxisEvents|InputAxisCameraVertical
  (params (AxisValue :type Float%20%28single-precision%29))
  (bind _returnvalue (Math|Rotator|MakeRotator 0.0 AxisValue 0.0))
  (bind _springarm (Variables|Default|GetSpringArm))
  (bind _returnvalue_2 (Class|SpringArmComponent|GetTargetRotation _springarm))
  (Transformation|AddRelativeRotation (Variables|Default|GetSpringArm) (Math|Rotator|MakeRotator (Math|Float|Clamp(Float) (.roll _returnvalue) 0.0 0.0) (.pitch _returnvalue) (.yaw (Math|Rotator|MakeRotator 0.0 0.0 (stale Input|AxisEvents|InputAxisCameraHorizontal AxisValue)))) false false)
  (Transformation|SetRelativeRotation _springarm (Math|Rotator|MakeRotator (.roll _returnvalue_2) (Math|Float|Clamp(Float) (.pitch _returnvalue_2) -75.0 75.0) (.yaw _returnvalue_2)) false false))

(event Input|AxisEvents|InputAxisCameraHorizontal
  (params (AxisValue :type Float%20%28single-precision%29))
  (bind _springarm (Variables|Default|GetSpringArm))
  (bind _returnvalue (Class|SpringArmComponent|GetTargetRotation _springarm))
  (Transformation|AddRelativeRotation (Variables|Default|GetSpringArm) (Math|Rotator|MakeRotator (Math|Float|Clamp(Float) (.roll (Math|Rotator|MakeRotator 0.0 (stale Input|AxisEvents|InputAxisCameraVertical AxisValue) 0.0)) 0.0 0.0) (.pitch (Math|Rotator|MakeRotator 0.0 (stale Input|AxisEvents|InputAxisCameraVertical AxisValue) 0.0)) (.yaw (Math|Rotator|MakeRotator 0.0 0.0 AxisValue))) false false)
  (Transformation|SetRelativeRotation _springarm (Math|Rotator|MakeRotator (.roll _returnvalue) (Math|Float|Clamp(Float) (.pitch _returnvalue) -75.0 75.0) (.yaw _returnvalue)) false false))

(event Input|AxisEvents|InputAxisMoveForward
  (params (AxisValue :type Float%20%28single-precision%29))
  (Class|PrimitiveComponent|AddTorqueinRadians (Variables|Default|GetBall) (* (* (Math|Vector|GetRightVector (Transformation|GetWorldRotation (Variables|Default|GetCamera))) AxisValue) (Variables|Default|GetBallTorque)) "None" false)
  (Physics|AddForce (Variables|Default|GetBall) (* (* (Math|Vector|GetForwardVector (Transformation|GetWorldRotation (Variables|Default|GetCamera))) AxisValue) (Variables|Default|GetForcePush)) "None" true))

(event Input|AxisEvents|InputAxisMoveRight
  (params (AxisValue :type Float%20%28single-precision%29))
  (Class|PrimitiveComponent|AddTorqueinRadians (Variables|Default|GetBall) (* (* (Math|Vector|GetForwardVector (Transformation|GetWorldRotation (Variables|Default|GetCamera))) AxisValue) (Variables|Default|GetBallTorque)) "None" false)
  (Physics|AddForce (Variables|Default|GetBall) (* (* (Math|Vector|GetRightVector (Transformation|GetWorldRotation (Variables|Default|GetCamera))) (* AxisValue -1.0)) (Variables|Default|GetForcePush)) "None" true))

(fn ConstructionScript)